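; Chained trigger box that drives story events in a VR game when the player overlaps it.
; Tick polls the overlap, then starts a subtitle or choice via BP_ChoiceSubtitleManager, plus optional seating, vision blur, scene-change FX and special events on actors, doors, environment and sounds.
; Once the manager stops playing, it waits DestroyDelay, enables the next triggers and destroys itself.
; Only boxes flagged FirstEventTrigger start enabled.
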(event EventBeginPlay
  ;[1 1 1] Set enabled or not depending on previous event trigger
  (if (Variables|Default|GetFirstEventTrigger)
    (CallFunction|SetEnabled)
    (else
      (CallFunction|SetHidden)))
  (bind _outactors (Actor|GetAllActorsOfClass "/Game/Bullied_VR/Blueprints/Subtitles/BP_ChoiceSubtitleManager.BP_ChoiceSubtitleManager_C"))
  (for _array_element _outactors
    (Variables|Default|SetCSManager _array_element)))

(event EventTick
  (params (DeltaSeconds :type Float%20%28single-precision%29))
  (bind _cameraeffectsref (Variables|Default|GetCameraEffectsRef))
  (bind _playerref (Variables|Default|GetPlayerRef))
  (bind _postprocess (Variables|Default|GetPostProcess))
  (bind _cameraeffectsref_2 (Variables|Default|GetCameraEffectsRef))
  (bind _environment (Variables|Default|GetEnvironment))
  (bind _disable_motion_ (Variables|Default|GetDisable%20Motion?))
  (bind _csmanager (Variables|Default|GetCSManager))
  ;[1 1 1] Check if checkpoint has been triggered before
  (if (Variables|Default|Getb_Triggered)
    ;[1 1 1] Check if it is ready to be destroyed
    (if (Variables|Default|Getb_Destroying)
      ;[1 1 1] Destroy and spawn next EventTriggers
      (bind _output_get (Variables|Default|Setf_elapseTime (+ (Variables|Default|Getf_elapseTime) (Utilities|Time|GetWorldDeltaSeconds))))
      (if (>= _output_get (Variables|Default|GetDestroyDelay))
        (for _array_element (Variables|Default|GetNextEventTrigger)
          (Utilities|IsValid _array_element
            (:Is%20Valid
              (CallFunction|SetEnabled _array_element))))
        (Actor|DestroyActor))
      (else
        ;[1 1 1] Get Ready to destroy
        (if (not (Variables|/Game/Bullied_VR/Blueprints/Subtitles/BP_ChoiceSubtitleManager.BP_ChoiceSubtitleManager_C|GetIsPlaying (Variables|Default|GetCSManager)))
          (Variables|Default|Setb_Destroying true)
          (if (Variables|Default|GetSceneChangeAfter?)
            (Utilities|IsValid _cameraeffectsref_2
              (:Is%20Valid
                (Default|SceneChangeFX _cameraeffectsref_2 2.0)))))))
    (else
      ;[1 1 1] Check if player has collided
      (if (Class|PrimitiveComponent|IsOverlappingComponent (Variables|Default|GetBoxCollision) (Variables|/Script/Engine.Character|GetCapsuleComponent (Variables|Default|GetPlayerRef)))
        (Utilities|FlowControl|Sequence
          (:then_0
            ;[1 1 1] Activate Subtitle / Choice
            (if (Variables|Default|GetIsChoice)
              (Default|ActivateChoice _csmanager (Variables|Default|GetChoice) _disable_motion_)
              (elif (Variables|Default|GetIsSubtitle)
                (Default|ActivateSubtitle _csmanager (Variables|Default|GetSubtitle) (Variables|Default|GetChoiceAfterSubtitle) (Variables|Default|GetChoice) _disable_motion_ self)))
            (Variables|Default|Setb_Triggered true))
          (:then_1
            ;[1 1 1] Make player sit or stand
            (if (Variables|Default|GetMake%20Player%20Sit?)
              (Default|PlayerSit _playerref)
              (CallFunction|MovePlayertoChair)
              (else
                (Default|PlayerStand _playerref))))
          (:then_2
            ;[1 1 1] Blur Player's vision on this event
            (if (Variables|Default|GetBlur%20Player%20Vision?)
              (Variables|/Script/Engine.PostProcessComponent|SetbEnabled _postprocess true)
              (Variables|/Script/Engine.PostProcessComponent|SetBlendWeight _postprocess 1.0)))
          (:then_3
            ;[1 1 1] Blink player eye on start
            (if (Variables|Default|GetSceneChangeBefore?)
              (Utilities|IsValid _cameraeffectsref
                (:Is%20Valid
                  (Default|SceneChangeFX _cameraeffectsref 2.0)))))
          (:then_4
            ;[1 1 1] Play Extra Special Event Effects
            (if (Variables|Default|GetPlaySpecialEvent?)
              (Utilities|FlowControl|Sequence
                (:then_0
                  (CallFunction|HideActors))
                (:then_1
                  (CallFunction|ShowActors))
                (:then_2
                  (CallFunction|CloseDoors))
                (:then_3
                  (CallFunction|UnlockDoors))
                (:then_4
                  (Utilities|IsValid _environment
                    (:Is%20Valid
                      (Utilities|FlowControl|Sequence
                        (:then_0
                          (if (Variables|Default|GetMoveEnvironment)
                            (Variables|/Game/Bullied_VR/Blueprints/BP_MovingEnviroment.BP_MovingEnviroment_C|SetIsMoving _environment true)))
                        (:then_1
                          (if (Variables|Default|GetStopEnvironment)
                            (Variables|/Game/Bullied_VR/Blueprints/BP_MovingEnviroment.BP_MovingEnviroment_C|SetIsMoving _environment false)))))))
                (:then_5
                  (CallFunction|PauseSounds))
                (:then_6
                  (CallFunction|PlaySounds))))))))))

(fn ConstructionScript)

(fn SetEnabled
  (Collision|SetActorEnableCollision true)
  (Rendering|SetActorHiddenInGame false)
  (Actor|Tick|SetActorTickEnabled true))

(fn SetHidden
  (Collision|SetActorEnableCollision false)
  (Rendering|SetActorHiddenInGame true)
  (Actor|Tick|SetActorTickEnabled false))

(fn MovePlayertoChair
  (bind _playerref (Variables|Default|GetPlayerRef))
  (bind _defaultsceneroot (Variables|Default|GetDefaultSceneRoot))
  (bind _returnvalue (Transformation|GetWorldLocation _defaultsceneroot))
  (bind _capsulecomponent (Variables|/Script/Engine.Character|GetCapsuleComponent _playerref))
  (bind (_x _y) (Math|Vector|BreakVector _returnvalue))
  (Transformation|SetWorldLocation _capsulecomponent (Math|Vector|MakeVector _x _y (.Z (Math|Vector|BreakVector (Transformation|GetWorldLocation _capsulecomponent)))) false false))

(fn HideActors
  (for _array_element (Variables|Default|GetActorsToHide)
    (Rendering|SetActorHiddenInGame _array_element true)
    (Collision|SetActorEnableCollision _array_element false)
    (Actor|Tick|SetActorTickEnabled _array_element)))

(fn ShowActors
  (for _array_element (Variables|Default|GetActorsToShow)
    (Rendering|SetActorHiddenInGame _array_element false)
    (Collision|SetActorEnableCollision _array_element true)
    (Actor|Tick|SetActorTickEnabled _array_element true)))

(fn CloseDoors
  (for _array_element (Variables|Default|GetDoorsToClose)
    (bind _asbp_interface_door (Utilities|Casting|CastToBP_InterfaceDoor _array_element))
    (Default|CloseDoor _asbp_interface_door)
    (if (Variables|Default|GetLockClosingDoor?)
      (Default|LockDoor _asbp_interface_door))))

(fn UnlockDoors
  (for _array_element (Variables|Default|GetDoorsToUnlock)
    (bind _asbp_interface_door (Utilities|Casting|CastToBP_InterfaceDoor _array_element))
    (Default|UnlockDoor _asbp_interface_door)))

(fn PauseSounds
  (for _array_element (Variables|Default|GetSoundsToPause)
    (Audio|Components|Audio|FadeOut (Variables|/Script/Engine.AmbientSound|GetAudioComponent _array_element) 1.0 0.0 :!class /Script/Engine.AudioComponent)))

(fn PlaySounds
  (for _array_element (Variables|Default|GetSoundsToPlay)
    (Audio|Components|Audio|Play (Variables|/Script/Engine.AmbientSound|GetAudioComponent _array_element) 0.0)))