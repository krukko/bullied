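; Choice controller that shows the player a dialogue-style list of options and handles navigating and confirming one.
; StartChoiceSelection takes the player character's choice widget, fills the HUD_ChoiceList, highlights the first entry and optionally disables motion.
; Up and down functions move the highlight within the list bounds.
; SelectChoice restores motion, closes the list and starts the choice's subtitle sequence through ChoiceSubManager if it has one.
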(event Custom|ChoiceSelected
  (bind _w_choicewidget (Variables|Default|GetW_ChoiceWidget))
  (if (not (Variables|/Game/Bullied_VR/Blueprints/NEWBlueprints/PlayerCharacter.PlayerCharacter_C|Getb_inChoice (Variables|Default|GetA_PlayerRef)))
    (Widget|SetVisibility _w_choicewidget "Hidden")
    (bind _ashud_choice_list (Utilities|Casting|CastToHUD_ChoiceList _w_choicewidget))
    (Default|OnFinish _ashud_choice_list)))

(fn ConstructionScript)

(fn ChangeChoiceUp
  (bind _choiceindex (Variables|Default|GetChoiceIndex))
  (bind _choiceindex_2 (Variables|Default|GetChoiceIndex))
  (bind _ashud_choice_list (Utilities|Casting|CastToHUD_ChoiceList (Variables|Default|GetW_ChoiceWidget)))
  (Math|Integer|CompareInt _choiceindex
    (:>
      (bind _ashud_choice_selection (Utilities|Casting|CastToHUD_ChoiceSelection (Class|PanelWidget|GetChildat (Variables|Default|GetW_ChoiceWidgetHBox) _choiceindex)))
      (Variables|/Game/Bullied_VR/Blueprints/NEWBlueprints/HUD_ChoiceSelection.HUD_ChoiceSelection_C|SetB_Selected _ashud_choice_selection false)
      (Default|ChangeChoice _ashud_choice_list _choiceindex_2)
      (bind _result (Math|Integer|DecrementInt _choiceindex_2)
        (:%20%20
          (bind _ashud_choice_selection_2 (Utilities|Casting|CastToHUD_ChoiceSelection (Class|PanelWidget|GetChildat (Variables|Default|GetW_ChoiceWidgetHBox) _result)))
          (Variables|/Game/Bullied_VR/Blueprints/NEWBlueprints/HUD_ChoiceSelection.HUD_ChoiceSelection_C|SetB_Selected _ashud_choice_selection_2 true)
          (Default|ChangeChoice _ashud_choice_list _result)
          (Development|PrintString "choiceup"))))))

(fn ChangeChoiceDown
  (bind _choiceindex (Variables|Default|GetChoiceIndex))
  (bind _w_choicewidgethbox (Variables|Default|GetW_ChoiceWidgetHBox))
  (bind _choiceindex_2 (Variables|Default|GetChoiceIndex))
  (bind _ashud_choice_list (Utilities|Casting|CastToHUD_ChoiceList (Variables|Default|GetW_ChoiceWidget)))
  (Math|Integer|CompareInt _choiceindex (- (Class|PanelWidget|GetChildrenCount _w_choicewidgethbox) 1)
    (:<
      (bind _ashud_choice_selection (Utilities|Casting|CastToHUD_ChoiceSelection (Class|PanelWidget|GetChildat _w_choicewidgethbox _choiceindex)))
      (Variables|/Game/Bullied_VR/Blueprints/NEWBlueprints/HUD_ChoiceSelection.HUD_ChoiceSelection_C|SetB_Selected _ashud_choice_selection false)
      (Default|ChangeChoice _ashud_choice_list _choiceindex_2)
      (bind _result (Math|Integer|IncrementInt _choiceindex_2)
        (:%20%20
          (bind _ashud_choice_selection_2 (Utilities|Casting|CastToHUD_ChoiceSelection (Class|PanelWidget|GetChildat (Variables|Default|GetW_ChoiceWidgetHBox) _result)))
          (Variables|/Game/Bullied_VR/Blueprints/NEWBlueprints/HUD_ChoiceSelection.HUD_ChoiceSelection_C|SetB_Selected _ashud_choice_selection_2 true)
          (Default|ChangeChoice _ashud_choice_list _result)
          (Development|PrintString "choicedown"))))))

(fn SelectChoice
  (bind _a_playerref (Variables|Default|GetA_PlayerRef))
  (bind _choicesubmanager (Variables|Default|GetChoiceSubManager))
  (bind _choiceindex (Variables|Default|GetChoiceIndex))
  (bind _ashud_choice_list (Utilities|Casting|CastToHUD_ChoiceList (Variables|Default|GetW_ChoiceWidget)))
  (bind _ashud_choice_selection (Utilities|Casting|CastToHUD_ChoiceSelection (Class|PanelWidget|GetChildat (Variables|/Game/Bullied_VR/Blueprints/NEWBlueprints/HUD_ChoiceList.HUD_ChoiceList_C|GetHBox _ashud_choice_list) _choiceindex)))
  (Default|SelectChoice _ashud_choice_list _choiceindex)
  (Variables|/Game/Bullied_VR/Blueprints/NEWBlueprints/PlayerCharacter.PlayerCharacter_C|Setb_inChoice _a_playerref false)
  (Variables|/Game/Bullied_VR/Blueprints/NEWBlueprints/PlayerCharacter.PlayerCharacter_C|Setb_DisableMotion _a_playerref false)
  (CallFunction|ChoiceSelected)
  (if (.HasSubtitles (Utilities|Struct|BreakChoiceInfo (Variables|/Game/Bullied_VR/Blueprints/NEWBlueprints/HUD_ChoiceSelection.HUD_ChoiceSelection_C|GetA_ChoiceInfo _ashud_choice_selection)))
    (Default|StartSubtitleSequence (Variables|/Game/Bullied_VR/Blueprints/NEWBlueprints/BP_ChoiceSubManager.BP_ChoiceSubManager_C|GetTextTriggerRef _choicesubmanager) (.Subtitles (Utilities|Struct|BreakChoiceInfo (Variables|/Game/Bullied_VR/Blueprints/NEWBlueprints/HUD_ChoiceSelection.HUD_ChoiceSelection_C|GetA_ChoiceInfo _ashud_choice_selection))) (.DisableMotion (Utilities|Struct|BreakChoiceInfo (Variables|/Game/Bullied_VR/Blueprints/NEWBlueprints/HUD_ChoiceSelection.HUD_ChoiceSelection_C|GetA_ChoiceInfo _ashud_choice_selection))))
    (Development|PrintString "Hello")
    (else
      (Variables|/Game/Bullied_VR/Blueprints/NEWBlueprints/BP_ChoiceSubManager.BP_ChoiceSubManager_C|Setb_IsPlaying _choicesubmanager false))))

(fn StartChoiceSelection
  (params (ChoiceInfo :type Array%20of%20Choice%20Info%20Structures) (DisableMotion :type Boolean))
  (bind _returnvalue (Game|GetPlayerController 0))
  (bind _returnvalue_2 (Pawn|GetControlledPawn _returnvalue))
  ;[1 1 1] Render the choice selection on screen
  (if (Utilities|ClassIsChildOf (Utilities|GetClass _returnvalue_2) "/Game/Bullied_VR/Blueprints/NEWBlueprints/PlayerCharacter.PlayerCharacter_C")
    (bind _asplayer_character (Utilities|Casting|CastToPlayerCharacter _returnvalue_2))
    (Variables|Default|SetA_PlayerRef _asplayer_character)
    (bind _output_get (Variables|Default|SetW_ChoiceWidget (Variables|/Game/Bullied_VR/Blueprints/NEWBlueprints/PlayerCharacter.PlayerCharacter_C|Getw_ChoiceWidget (Variables|Default|GetA_PlayerRef))))
    (Widget|SetVisibility (Variables|/Game/Bullied_VR/Blueprints/NEWBlueprints/PlayerCharacter.PlayerCharacter_C|Getw_ChoiceWidget (Variables|Default|GetA_PlayerRef)) "Visible")
    (Variables|/Game/Bullied_VR/Blueprints/NEWBlueprints/PlayerCharacter.PlayerCharacter_C|Setb_inChoice (Variables|Default|GetA_PlayerRef) true)
    (Variables|/Game/Bullied_VR/Blueprints/NEWBlueprints/PlayerCharacter.PlayerCharacter_C|Setb_DisableMotion (Variables|Default|GetA_PlayerRef) DisableMotion)
    (bind _ashud_choice_list (Utilities|Casting|CastToHUD_ChoiceList (Variables|/Game/Bullied_VR/Blueprints/NEWBlueprints/PlayerCharacter.PlayerCharacter_C|Getw_ChoiceWidget (Variables|Default|GetA_PlayerRef))))
    (Variables|/Game/Bullied_VR/Blueprints/NEWBlueprints/HUD_ChoiceList.HUD_ChoiceList_C|SetChoiceInfoArray _ashud_choice_list ChoiceInfo)
    (Default|OnCreate _ashud_choice_list)
    (Variables|Default|SetW_ChoiceWidget (Variables|/Game/Bullied_VR/Blueprints/NEWBlueprints/HUD_ChoiceList.HUD_ChoiceList_C|GetHBox _ashud_choice_list))
    (bind _ashud_choice_selection (Utilities|Casting|CastToHUD_ChoiceSelection (Class|PanelWidget|GetChildat (Variables|/Game/Bullied_VR/Blueprints/NEWBlueprints/HUD_ChoiceList.HUD_ChoiceList_C|GetHBox _ashud_choice_list))))
    (Variables|/Game/Bullied_VR/Blueprints/NEWBlueprints/HUD_ChoiceSelection.HUD_ChoiceSelection_C|SetB_Selected _ashud_choice_selection true)
    (Default|ChangeChoice _ashud_choice_list)
    (Development|PrintString "  choice changed")))