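; BP_LevelTransistion is a level exit trigger that fades the screen out and loads the next level.
; Tick polls whether the player reference overlaps the collision box, firing only when LastTrigger is no longer a valid object.
; It then starts a held camera fade and accumulates elapsed time until the fade duration passes, when it shows the splash screen and opens NextLevelName.
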(event EventTick
  (params (DeltaSeconds :type Float%20%28single-precision%29))
  ;[1 1 1] Fade out to next level
  (if (Variables|Default|Getb_Triggered)
    (bind _output_get (Variables|Default|Setf_ElapsedTime (+ (Variables|Default|Getf_ElapsedTime) DeltaSeconds)))
    (if (>= _output_get (Variables|Default|GetFadeOutTime))
      (Class|StereoLayerFunctionLibrary|ShowSplashScreen)
      (Game|OpenLevel(byName) (Variables|Default|GetNextLevelName)))
    (else
      ;[1 1 1] Check player is in collision box
      (if (Collision|IsOverlappingActor (Variables|Default|GetCollision%20Box) (Variables|Default|GetPlayerMCRef) :!class /Script/Engine.PrimitiveComponent)
        (Utilities|IsValid (Variables|Default|GetLast%20Trigger)
          (:Is%20Not%20Valid
            (CameraFades|StartCameraFade :self (Game|GetPlayerCameraManager 0) :ToAlpha 1.0 :Duration (Variables|Default|GetFadeOutTime) :bHoldWhenFinished true)
            (Variables|Default|Setb_Triggered true)))))))

(fn ConstructionScript)