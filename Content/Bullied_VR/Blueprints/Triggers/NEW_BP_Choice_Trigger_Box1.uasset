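; Choice trigger Blueprint that drives an on-screen dialogue choice list (HUD_ChoiceList) for the player.
; ChangeChoiceUp and ChangeChoiceDown move the highlighted HUD_ChoiceSelection within the list's bounds.
; SelectChoice commits the pick, releases the player's choice and motion flags, hides and finishes the widget, then starts the choice's subtitle sequence or clears CSManager's playing flag.
; StartChoiceSelection and FindActivePawn are empty, with their setup logic left disconnected.
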(event Custom|ChoiceSelected
  (bind _pchoicewidget (Variables|Default|GetPChoiceWIdget))
  ;[1 1 1] Check if player Trigger Choice Selection
  (if (not (Variables|/Game/Bullied_VR/Blueprints/Player/BP_MotionControllerPawnFPS.BP_MotionControllerPawnFPS_C|GetInChoice (Variables|Default|GetPlayerMCRef)))
    (Widget|SetVisibility _pchoicewidget "Hidden")
    (bind _ashud_choice_list (Utilities|Casting|CastToHUD_ChoiceList _pchoicewidget))
    (Default|OnFinish _ashud_choice_list)))

(fn ConstructionScript)

(fn ChangeChoiceUp
  (bind _choiceindex (Variables|Default|GetChoiceIndex))
  (bind _choiceindex_2 (Variables|Default|GetChoiceIndex))
  (bind _ashud_choice_list (Utilities|Casting|CastToHUD_ChoiceList (Variables|Default|GetPChoiceWIdget)))
  (Math|Integer|CompareInt _choiceindex
    (:>
      (bind _ashud_choice_selection (Utilities|Casting|CastToHUD_ChoiceSelection (Class|PanelWidget|GetChildat (Variables|Default|GetPChoiceWidgetHBox) _choiceindex)))
      (Variables|/Game/Bullied_VR/Blueprints/HUDs/HUD_ChoiceSelection.HUD_ChoiceSelection_C|SetSelected _ashud_choice_selection false)
      (Default|ChangeChoice _ashud_choice_list _choiceindex_2)
      (bind _result (Math|Integer|DecrementInt _choiceindex_2)
        (:%20%20
          (bind _ashud_choice_selection_2 (Utilities|Casting|CastToHUD_ChoiceSelection (Class|PanelWidget|GetChildat (Variables|Default|GetPChoiceWidgetHBox) _result)))
          (Variables|/Game/Bullied_VR/Blueprints/HUDs/HUD_ChoiceSelection.HUD_ChoiceSelection_C|SetSelected _ashud_choice_selection_2 true)
          (Default|ChangeChoice _ashud_choice_list _result))))))

(fn ChangeChoiceDown
  (bind _choiceindex (Variables|Default|GetChoiceIndex))
  (bind _pchoicewidgethbox (Variables|Default|GetPChoiceWidgetHBox))
  (bind _choiceindex_2 (Variables|Default|GetChoiceIndex))
  (bind _ashud_choice_list (Utilities|Casting|CastToHUD_ChoiceList (Variables|Default|GetPChoiceWIdget)))
  (Math|Integer|CompareInt _choiceindex (- (Class|PanelWidget|GetChildrenCount _pchoicewidgethbox) 1)
    (:<
      (bind _ashud_choice_selection (Utilities|Casting|CastToHUD_ChoiceSelection (Class|PanelWidget|GetChildat _pchoicewidgethbox _choiceindex)))
      (Variables|/Game/Bullied_VR/Blueprints/HUDs/HUD_ChoiceSelection.HUD_ChoiceSelection_C|SetSelected _ashud_choice_selection false)
      (Default|ChangeChoice _ashud_choice_list _choiceindex_2)
      (bind _result (Math|Integer|IncrementInt _choiceindex_2)
        (:%20%20
          (bind _ashud_choice_selection_2 (Utilities|Casting|CastToHUD_ChoiceSelection (Class|PanelWidget|GetChildat (Variables|Default|GetPChoiceWidgetHBox) _result)))
          (Variables|/Game/Bullied_VR/Blueprints/HUDs/HUD_ChoiceSelection.HUD_ChoiceSelection_C|SetSelected _ashud_choice_selection_2 true)
          (Default|ChangeChoice _ashud_choice_list _result))))))

(fn SelectChoice
  (bind _choiceindex (Variables|Default|GetChoiceIndex))
  (bind _playermcref (Variables|Default|GetPlayerMCRef))
  (bind _csmanager (Variables|Default|GetCSManager))
  (bind _ashud_choice_list (Utilities|Casting|CastToHUD_ChoiceList (Variables|Default|GetPChoiceWIdget)))
  (bind _ashud_choice_selection (Utilities|Casting|CastToHUD_ChoiceSelection (Class|PanelWidget|GetChildat (Variables|/Game/Bullied_VR/Blueprints/HUDs/HUD_ChoiceList.HUD_ChoiceList_C|GetHBox _ashud_choice_list) _choiceindex)))
  (Default|SelectChoice _ashud_choice_list _choiceindex)
  (Variables|/Game/Bullied_VR/Blueprints/Player/BP_MotionControllerPawnFPS.BP_MotionControllerPawnFPS_C|SetInChoice _playermcref false)
  (Variables|/Game/Bullied_VR/Blueprints/Player/BP_MotionControllerPawnFPS.BP_MotionControllerPawnFPS_C|SetDisableMotion _playermcref false)
  (CallFunction|ChoiceSelected)
  (if (.HasSubtitle (Utilities|Struct|BreakChoiceInfo (Variables|/Game/Bullied_VR/Blueprints/HUDs/HUD_ChoiceSelection.HUD_ChoiceSelection_C|GetChoiceInfo _ashud_choice_selection)))
    (Default|StartSubtitleSequence (Variables|/Game/Bullied_VR/Blueprints/Subtitles/BP_ChoiceSubtitleManager.BP_ChoiceSubtitleManager_C|GetTTB _csmanager) (.Subtitles (Utilities|Struct|BreakChoiceInfo (Variables|/Game/Bullied_VR/Blueprints/HUDs/HUD_ChoiceSelection.HUD_ChoiceSelection_C|GetChoiceInfo _ashud_choice_selection))) (.DisableMotion (Utilities|Struct|BreakChoiceInfo (Variables|/Game/Bullied_VR/Blueprints/HUDs/HUD_ChoiceSelection.HUD_ChoiceSelection_C|GetChoiceInfo _ashud_choice_selection))))
    (else
      (Variables|/Game/Bullied_VR/Blueprints/Subtitles/BP_ChoiceSubtitleManager.BP_ChoiceSubtitleManager_C|SetIsPlaying _csmanager false))))

(fn StartChoiceSelection
  (params (ChoiceArray :type Array%20of%20Choice%20Info%20Structures) (Disable%20Motion :type Boolean)))

(fn FindActivePawn)