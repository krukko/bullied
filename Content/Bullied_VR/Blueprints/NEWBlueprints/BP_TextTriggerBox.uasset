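; BP_TextTriggerBox drives subtitled dialogue, both for cutscenes and for interaction text with the player or AI.
; StartSubtitleSequence loads string table subtitles, audio and sequences; Tick waits for audio to finish, then plays the index's sequence or advances subtitle and sound.
; When subtitles run out, it can hand off to a choice selection.
; IterateText steps interaction text, pausing the AI's brain logic and rotating it until the text ends.
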(event Custom|OnStopEven0
  (Variables|Default|Setb_SequencePlaying false)
  (Utilities|Map|Remove (Variables|Default|Geta_Sequence) (Variables|Default|Geti_AudioIndex)))

(event EventTick
  (params (DeltaSeconds :type Float%20%28single-precision%29))
  (bind _a_sequence (Variables|Default|Geta_Sequence))
  (bind _a_sequence_2 (Variables|Default|Geta_Sequence))
  (bind _i_audioindex (Variables|Default|Geti_AudioIndex))
  (bind _audioplayer (Variables|Default|GetAudioPlayer))
  (bind _s_audio (Variables|Default|Gets_Audio))
  (bind _b_isplayingcutscene (Variables|Default|Getb_IsPlayingCutscene))
  (bind _i_audioindex_2 (Variables|Default|Geti_AudioIndex))
  (bind _b_isinteractingwithaudio (Variables|Default|Getb_isInteractingWithAudio))
  (bind _value (Utilities|Map|Find _a_sequence _i_audioindex_2))
  (bind _value_2 (Utilities|Map|Find _a_sequence_2 _i_audioindex))
  (bind _returnvalue (or _b_isinteractingwithaudio _b_isplayingcutscene))
  (bind _output (Utilities|Array|Get(acopy) _s_audio _i_audioindex))
  (bind (_audiofile _soundlocation) (Utilities|Struct|BreakSoundStruct _output))
  (bind _sequenceplayer (Variables|/Script/LevelSequence.LevelSequenceActor|GetSequencePlayer _value_2))
  (bind _sequenceplayer_2 (Variables|/Script/LevelSequence.LevelSequenceActor|GetSequencePlayer _value))
  (if _returnvalue
    (bind _array_element (Utilities|Array|ForEachLoopwithBreak (Variables|Default|Gets_ActorsInScene) :!label _label)
      (:LoopBody
        (Utilities|IsValid _array_element
          (:Is%20Valid
            (bind _output_get (Variables|Default|Setb_isAudioPlaying (Audio|Components|Audio|IsPlaying (Variables|/Game/Bullied_VR/Blueprints/NEWBlueprints/BP_SoundLocation.BP_SoundLocation_C|GetAudioPlayer _array_element))))
            (if _output_get
              (goto _label Break)))))
      (:Completed
        (if (not (or (Audio|Components|Audio|IsPlaying (Variables|Default|GetAudioPlayer)) (Variables|Default|Getb_isAudioPlaying)))
          (if (not (Variables|Default|Getb_SequencePlaying))
            (if (Utilities|Map|Contains _a_sequence_2 _i_audioindex)
              (Sequencer|Player|Play _sequenceplayer :!class /Script/MovieScene.MovieSceneSequencePlayer)
              (Variables|Default|Setb_SequencePlaying (Audio|Components|Audio|IsPlaying _sequenceplayer))
              (EventDispatchers|BindEventtoOnStop _sequenceplayer (delegate Custom|OnStopEven0))
              (else
                (CallFunction|PlayCutsceneSub)
                (if _returnvalue
                  (Utilities|IsValid _soundlocation
                    (:Is%20Not%20Valid
                      (Audio|Components|Audio|SetSound _audioplayer _audiofile)
                      (Audio|Components|Audio|Play _audioplayer 0.0)
                      (Math|Integer|CompareInt _i_audioindex (- (Utilities|Array|Length _s_audio) 1)
                        (:==
                          _)
                        (:<
                          _))
                      (Math|Integer|IncrementInt (Variables|Default|Geti_AudioIndex)))))))))))
    (else
      (Math|Integer|CompareInt (Utilities|Map|Length _a_sequence)
        (:>
          (if (not (Variables|Default|Getb_SequencePlaying))
            (Sequencer|Player|Play _sequenceplayer_2 :!class /Script/MovieScene.MovieSceneSequencePlayer)
            (Variables|Default|Setb_SequencePlaying (Audio|Components|Audio|IsPlaying _sequenceplayer_2))
            (EventDispatchers|BindEventtoOnStop _sequenceplayer_2 (delegate Custom|OnStopEven0))))))))

(fn ConstructionScript)

(fn IterateText
  (bind _a_interacttextarray (Variables|Default|Geta_InteractTextArray))
  (bind _c_playerref (Variables|Default|GetC_PlayerRef))
  (if (Variables|Default|Getb_IsInteracting)
    (Utilities|IsValid (Variables|Default|Geta_InteractingAI)
      (:Is%20Valid
        (AI|Logic|StopLogic (Variables|/Script/AIModule.AIController|GetBrainComponent (AI|GetAIController (Variables|Default|Geta_InteractingAI))) ""))
      (:Is%20Not%20Valid
        _))
    (Transformation|SetActorRotation (Variables|Default|Geta_InteractingAI) (Math|Rotator|FindLookatRotation (Transformation|GetActorLocation (Game|GetPlayerCharacter 0)) (Transformation|GetActorLocation (Variables|Default|Geta_InteractingAI))))
    (if (Utilities|IsValid (Variables|Default|Geta_InteractingAI))
      (bind _assubtitle_widget (Utilities|Casting|CastToSubtitleWidget (Variables|Default|GetW_SubtitleRef)))
      (Math|Integer|CompareInt (Variables|Default|Geti_SubtitleIndex) (- (Utilities|Array|Length _a_interacttextarray) 1)
        (:>
          (Variables|/Game/Bullied_VR/Blueprints/NEWBlueprints/PlayerCharacter.PlayerCharacter_C|Setb_DisableMotion _c_playerref false)
          (Default|DisplaySubtitleText _assubtitle_widget false)
          (Variables|Default|Seti_SubtitleIndex 0)
          (if (Utilities|IsValid (Variables|Default|Geta_InteractingAI))
            (Utilities|IsValid (Variables|Default|Geta_InteractingAI)
              (:Is%20Valid
                (Class|BrainComponent|RestartLogic (Variables|/Script/AIModule.AIController|GetBrainComponent (AI|GetAIController (Variables|Default|Geta_InteractingAI))))
                (Variables|Default|Seta_InteractingAI 0))
              (:Is%20Not%20Valid
                _)))
          (Variables|Default|Setb_IsInteracting false))
        (:==
          (Default|SetSubtitleText _assubtitle_widget (Utilities|Array|Get(acopy) _a_interacttextarray) :!label _label)
          (Default|DisplaySubtitleText _assubtitle_widget true)
          (Math|Integer|IncrementInt (Variables|Default|Geti_SubtitleIndex)
            (:%20%20
              (Variables|/Game/Bullied_VR/Blueprints/NEWBlueprints/PlayerCharacter.PlayerCharacter_C|Setb_DisableMotion _c_playerref false))))
        (:<
          (goto _label))))))

(fn PlayCutsceneSub
  (bind _a_subtitletext (Variables|Default|Geta_SubtitleText))
  (bind _c_choicesubmanager (Variables|Default|Getc_ChoiceSubManager))
  (bind _assubtitle_widget (Utilities|Casting|CastToSubtitleWidget (Variables|Default|GetW_SubtitleRef)))
  (Math|Integer|CompareInt (Variables|Default|Geti_SubtitleIndex) (- (Utilities|Array|Length _a_subtitletext) 1)
    (:>
      (Default|DisplaySubtitleText _assubtitle_widget false)
      (Variables|Default|Seti_SubtitleIndex 0)
      (Variables|Default|Seti_AudioIndex 0)
      (Variables|Default|Setb_IsPlayingCutscene false)
      (if (Variables|Default|Getb_StartChoiceAfter)
        (Default|StartChoiceSelection (Variables|/Game/Bullied_VR/Blueprints/NEWBlueprints/BP_ChoiceSubManager.BP_ChoiceSubManager_C|GetChoiceTriggerRef _c_choicesubmanager) (Variables|Default|GetA_Choice) true)
        (Variables|Default|Setb_StartChoiceAfter false)
        (Development|PrintString "Hello")
        (else
          (Variables|/Game/Bullied_VR/Blueprints/NEWBlueprints/BP_ChoiceSubManager.BP_ChoiceSubManager_C|Setb_IsPlaying _c_choicesubmanager false))))
    (:==
      (Default|SetSubtitleText _assubtitle_widget (Utilities|Array|Get(acopy) _a_subtitletext (Variables|Default|Geti_SubtitleIndex)) :!label _label)
      (Default|DisplaySubtitleText _assubtitle_widget true)
      (Math|Integer|IncrementInt (Variables|Default|Geti_SubtitleIndex)))
    (:<
      (goto _label))))

(fn SetSubText
  (params (StringTableName :type Name))
  (bind _a_subtitletext (Variables|Default|Geta_SubtitleText))
  (Utilities|Array|Clear _a_subtitletext)
  (for (_ _array_index) (Class|KismetStringTableLibrary|GetKeysfromStringTable StringTableName)
    (Utilities|Array|Add _a_subtitletext (Utilities|String|ToString(Text) (Class|KismetTextLibrary|TextfromStringTable StringTableName (Utilities|String|ToString(Integer) _array_index))))))

(fn SetInteractText
  (params (TextArray :type Array%20of%20Strings) (HasAudio :type Boolean))
  (Utilities|Array|Clear (Variables|Default|Geta_InteractTextArray))
  (Utilities|Array|Clear (Variables|Default|Geta_SubtitleText))
  (if HasAudio
    (Variables|Default|Seta_SubtitleText TextArray)
    (else
      (Variables|Default|Seta_InteractTextArray TextArray))))

(fn StartAIInteractionText
  (params (a_InteractingAI :type Actor%20Object%20Reference) (TextArray :type Array%20of%20Strings))
  (Variables|Default|Seta_InteractingAI a_InteractingAI)
  (CallFunction|SetInteractText TextArray false)
  (bind _asplayer_character (Utilities|Casting|CastToPlayerCharacter (Game|GetPlayerCharacter 0)))
  (Variables|Default|Setw_SubtitleRef (Variables|/Game/Bullied_VR/Blueprints/NEWBlueprints/PlayerCharacter.PlayerCharacter_C|Getw_SubtitleWidget _asplayer_character))
  (Variables|Default|SetC_PlayerRef _asplayer_character)
  (Variables|Default|Setb_IsInteracting true))

(fn StartInteractionText
  (params (TextArray :type Array%20of%20Strings) (HasAudio :type Boolean))
  (CallFunction|SetInteractText TextArray HasAudio)
  (bind _asplayer_character (Utilities|Casting|CastToPlayerCharacter (Game|GetPlayerCharacter 0)))
  (Variables|Default|SetW_SubtitleRef (Variables|/Game/Bullied_VR/Blueprints/NEWBlueprints/PlayerCharacter.PlayerCharacter_C|Getw_SubtitleWidget _asplayer_character))
  (Variables|Default|SetC_PlayerRef _asplayer_character)
  (bind _output_get (Variables|Default|Setb_IsInteracting HasAudio))
  (if _output_get
    (CallFunction|IterateText)))

(fn StartSubtitleSequence
  (params (SubInfo :type Subtitle%20Info%20Structure) (DisableMotion :type Boolean))
  (bind (_audioarray _stringtableref _sequencearray) (Utilities|Struct|BreakSubtitleInfo SubInfo))
  (bind _s_actorsinscene (Variables|Default|Gets_ActorsInScene))
  (if (not (Variables|Default|Getb_IsPlayingCutscene))
    (CallFunction|SetSubText (.OutTableId (Class|KismetTextLibrary|StringTableIdandKeyfromText _stringtableref)))
    (bind _output_get (Variables|Default|SetS_Audio _audioarray))
    (Utilities|Array|Clear _s_actorsinscene)
    (for _array_element _output_get
      (Utilities|Array|Add _s_actorsinscene (.SoundLocation (Utilities|Struct|BreakSoundStruct _array_element))))
    (Variables|Default|Setb_IsPlayingCutscene true)
    (bind _asplayer_character (Utilities|Casting|CastToPlayerCharacter (Game|GetPlayerCharacter 0)))
    (Variables|Default|SetW_SubtitleRef (Variables|/Game/Bullied_VR/Blueprints/NEWBlueprints/PlayerCharacter.PlayerCharacter_C|Getw_SubtitleWidget _asplayer_character))
    (Variables|Default|SetC_PlayerRef 0)
    (Variables|/Game/Bullied_VR/Blueprints/NEWBlueprints/PlayerCharacter.PlayerCharacter_C|Setb_DisableMotion _asplayer_character DisableMotion)
    (Variables|Default|Seta_Sequence _sequencearray)))