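; BP_LookableActor is an actor in Bullied_VR that shows interaction text when triggered by the player's look.
; LookTrigger casts the caller to PlayerCharacter, stores it and runs StartInteraction once until re-armed.
; StartInteraction passes InteractText without audio to TextTriggerRef, flags it as interacting and prints a debug "Hello".
; The HasTriggered latch clears when that stored player ends overlap with the actor.
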(event EventBeginPlay)

(event EventLookTrigger
  (params (Player's%20MCRef :type Actor%20Object%20Reference))
  (if (not (Variables|Default|GetHasTriggered))
    (bind _asplayer_character (Utilities|Casting|CastToPlayerCharacter Player's%20MCRef))
    (Variables|Default|SetPlayerMCRef _asplayer_character)
    (CallFunction|StartInteraction)))

(event Collision|EventActorEndOverlap
  (params (OtherActor :type Actor%20Object%20Reference))
  (if (Variables|Default|GetHasTriggered)
    (if (== OtherActor (Variables|Default|GetPlayerMCRef))
      (Variables|Default|SetHasTriggered false))))

(fn ConstructionScript)

(fn StartInteraction
  (bind _texttriggerref (Variables|Default|GetTextTriggerRef))
  (Default|StartInteractionText _texttriggerref (Variables|Default|GetInteractText) false)
  (Variables|/Game/Bullied_VR/Blueprints/NEWBlueprints/BP_TextTriggerBox.BP_TextTriggerBox_C|Setb_isInteracting _texttriggerref true)
  (Variables|Default|SetHasTriggered true)
  (Development|PrintString "Hello"))