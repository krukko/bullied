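; Chained trigger box that starts a subtitle or choice through BP_ChoiceSubManager when a pawn overlaps it, optionally blurring vision or seating the player.
; Only the first trigger starts enabled; each polls overlap on Tick.
; Once the manager stops playing, it can fire a scene-change effect, then enables the next triggers and destroys itself after a delay that only advances during overlap.
; Door and sound helpers are defined but never called here.
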(event Custom|EventTriggered
  (bind _b_disablemotion (Variables|Default|Getb_DisableMotion))
  (bind _a_camerafxref (Variables|Default|GetA_CameraFXRef))
  (bind _bp_choicesubmanager (Variables|Default|GetBP_ChoiceSubManager))
  (bind _postprocess (Variables|Default|GetPostProcess))
  (if (Variables|Default|Getb_Triggered)
    (if (Variables|Default|Getb_isDestroying)
      ;[1 1 1] Destroy the previous trigger and spawn the new one
      (Development|PrintString "nya")
      (bind _output_get (Variables|Default|Setf_ElapseTime (+ (Variables|Default|Getf_ElapseTime) (Utilities|Time|GetWorldDeltaSeconds))))
      (if (>= _output_get (Variables|Default|Getf_DestroyDelay))
        (for _array_element (Variables|Default|GetA_NextEventTrigger)
          (Utilities|IsValid _array_element
            (:Is%20Valid
              (CallFunction|SetEnabled _array_element))))
        (Actor|DestroyActor)
        (Development|PrintString "destroy"))
      (else
        ;[1 1 1] Prepare to destroy...!
        (if (not (Variables|/Game/Bullied_VR/Blueprints/NEWBlueprints/BP_ChoiceSubManager.BP_ChoiceSubManager_C|Getb_IsPlaying (Variables|Default|GetBP_ChoiceSubManager)))
          (Variables|Default|Setb_isDestroying true)
          (if (Variables|Default|Getb_ChangeSceneBefore)
            (Utilities|IsValid _a_camerafxref
              (:Is%20Valid
                (Default|SceneChangeFX _a_camerafxref 1.0)))))))
    (else
      (Utilities|FlowControl|Sequence
        (:then_0
          ;[1 1 1] Activate subtitle/choice
          (if (Variables|Default|Getb_IsChoice)
            (Default|ActivateChoice _bp_choicesubmanager (Variables|Default|Geta_ChoiceRef) _b_disablemotion)
            (elif (Variables|Default|Getb_IsSubtitle)
              (Default|ActivateSubtitle _bp_choicesubmanager (Variables|Default|Geta_SubReference) _b_disablemotion (Variables|Default|Getb_ChoiceAfterSub) (Variables|Default|Geta_ChoiceRef) self)))
          (Variables|Default|Setb_Triggered true))
        (:then_1
          ;[1 1 1] Blur player's vision
          (if (Variables|Default|Getb_BlurPlayerVision)
            (Variables|/Script/Engine.PostProcessComponent|SetbEnabled _postprocess true)
            (Variables|/Script/Engine.PostProcessComponent|SetBlendWeight _postprocess 1.0)))
        (:then_2
          ;[1 1 1] Blink at the start of the scene
          (if (Variables|Default|Getb_ChangeSceneBefore)
            (Utilities|IsValid (Variables|Default|Geta_CameraFXRef))))
        (:then_3
          ;[1 1 1] Make player sit or stand in the scene
          (if (Variables|Default|Getb_MakePlayerSit)
            (Default|SitDown (Variables|Default|Geta_PlayerRef))
            (CallFunction|MovePlayertoChair)))))))

(event EventBeginPlay
  ;[1 1 1] Set Enabled/Disabled based on the previous event trigger
  (if (Variables|Default|Getb_FirstEventTrigger)
    (CallFunction|SetEnabled)
    (else
      (CallFunction|SetHidden)))
  (bind _outactors (Actor|GetAllActorsOfClass "/Game/Bullied_VR/Blueprints/NEWBlueprints/BP_ChoiceSubManager.BP_ChoiceSubManager_C"))
  (for _array_element _outactors
    (Variables|Default|SetBP_ChoiceSubManager _array_element)))

(event EventTick
  (params (DeltaSeconds :type Float%20%28single-precision%29))
  ;[1 1 1] Check whether the player has collided with the trigger
  (bind _returnvalue (Collision|ComponentOverlapActors (Variables|Default|GetBoxCollision) (Transformation|GetWorldTransform (Variables|Default|GetDefaultSceneRoot)) (Utilities|Array|MakeArray "ObjectTypeQuery3") 0))
  (if _returnvalue
    (CallFunction|EventTriggered)))

(fn ConstructionScript)

(fn SetEnabled
  (Collision|SetActorEnableCollision false)
  (Rendering|SetActorHiddenInGame false)
  (Actor|Tick|SetActorTickEnabled true))

(fn SetHidden
  (Collision|SetActorEnableCollision false)
  (Rendering|SetActorHiddenInGame true)
  (Actor|Tick|SetActorTickEnabled false))

(fn CloseDoors
  (for _array_element (Variables|Default|GetA_DoorsToClose)
    (bind _asbp_door_interface (Utilities|Casting|CastToBP_DoorInterface _array_element))
    (if true
      (Default|LockDoor _asbp_door_interface))))

(fn HideActors)

(fn MovePlayertoChair
  (bind _a_playerref (Variables|Default|GetA_PlayerRef))
  (bind _defaultsceneroot (Variables|Default|GetDefaultSceneRoot))
  (bind _returnvalue (Transformation|GetWorldLocation _defaultsceneroot))
  (bind _rootcomponent (Variables|/Script/Engine.Actor|GetRootComponent _a_playerref))
  (bind (_x _y) (Math|Vector|BreakVector _returnvalue))
  (Transformation|SetWorldLocation _rootcomponent (Math|Vector|MakeVector _x _y (.Z (Math|Vector|BreakVector (Transformation|GetWorldLocation _rootcomponent)))) false false))

(fn PauseSounds
  (for _array_element (Variables|Default|GetA_SoundsToPause)
    (Audio|Components|Audio|FadeOut (Variables|/Script/Engine.AmbientSound|GetAudioComponent _array_element) 1.0 0.0 :!class /Script/Engine.AudioComponent)))

(fn PlaySounds
  (for _array_element (Variables|Default|GetA_SoundsToPlay)
    (Audio|Components|Audio|Play (Variables|/Script/Engine.AmbientSound|GetAudioComponent _array_element) 0.0)))