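; BP_ChoiceSubManager is a manager that starts subtitle sequences and dialogue choices and routes player input to them.
; ActivateSubtitle and ActivateChoice forward data to the text and choice triggers, and a subtitle can queue a choice to follow.
; Tick, throttled by a Delay, polls flags on the player found at BeginPlay: trigger and scroll inputs select or change choices during cutscenes, while scroll-up otherwise advances interactive text.
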(event EventBeginPlay
  (bind _outactors (Actor|GetAllActorsOfClass "/Game/Bullied_VR/Blueprints/NEWBlueprints/PlayerCharacter.PlayerCharacter_C"))
  (bind _array_element (Utilities|Array|ForEachLoopwithBreak _outactors :!label _label)
    (:LoopBody
      (Variables|Default|SetA_PlayerRef _array_element)
      (goto _label Break))))

(event EventTick
  (params (DeltaSeconds :type Float%20%28single-precision%29))
  (bind _a_playerref (Variables|Default|GetA_PlayerRef))
  (bind _texttriggerref (Variables|Default|GetTextTriggerRef))
  (bind _choicetriggerref (Variables|Default|GetChoiceTriggerRef))
  (bind _scrollup (Variables|/Game/Bullied_VR/Blueprints/NEWBlueprints/PlayerCharacter.PlayerCharacter_C|GetScrollUp _a_playerref))
  (Utilities|FlowControl|Delay 0.2)
  (if (Variables|/Game/Bullied_VR/Blueprints/NEWBlueprints/PlayerCharacter.PlayerCharacter_C|GetCSM_Do_Action _a_playerref)
    (if (Variables|/Game/Bullied_VR/Blueprints/NEWBlueprints/BP_TextTriggerBox.BP_TextTriggerBox_C|Getb_IsPlayingCutscene _texttriggerref)
      (if (Variables|/Game/Bullied_VR/Blueprints/NEWBlueprints/PlayerCharacter.PlayerCharacter_C|Getb_inChoice _a_playerref)
        (Utilities|FlowControl|Sequence
          (:then_0
            (if (Variables|/Game/Bullied_VR/Blueprints/NEWBlueprints/PlayerCharacter.PlayerCharacter_C|Getb_TriggerLeftDown _a_playerref)
              (Default|SelectChoice _choicetriggerref)))
          (:then_1
            (if _scrollup
              (Default|ChangeChoiceUp _choicetriggerref)))
          (:then_2
            (if (Variables|/Game/Bullied_VR/Blueprints/NEWBlueprints/PlayerCharacter.PlayerCharacter_C|GetScrollDown _a_playerref)
              (Default|ChangeChoiceDown _choicetriggerref))))
        (elif _scrollup
          (if (Variables|/Game/Bullied_VR/Blueprints/NEWBlueprints/BP_TextTriggerBox.BP_TextTriggerBox_C|Getb_IsInteracting _texttriggerref)
            (Default|IterateText _texttriggerref)))))))

(fn ConstructionScript)

(fn ActivateChoice
  (params (ChoiceInfo :type Array%20of%20Choice%20Info%20Structures) (DisableMotion :type Boolean))
  (Default|StartChoiceSelection (Variables|Default|GetChoiceTriggerRef) ChoiceInfo DisableMotion)
  (Variables|Default|Setb_IsPlaying true))

(fn ActivateSubtitle
  (params (SubtitleInfo :type Subtitle%20Info%20Structure) (DisableMotion :type Boolean) (StartChoiceAfter :type Boolean) (ChoiceArray :type Array%20of%20Choice%20Info%20Structures) (CurrentEventTrBox :type BP%20Event%20Trigger%20Box%20Object%20Reference))
  (bind _texttriggerref (Variables|Default|GetTextTriggerRef))
  (Default|StartSubtitleSequence _texttriggerref SubtitleInfo DisableMotion)
  (Variables|Default|Seta_CurrentEventTrgBox CurrentEventTrBox)
  (Variables|Default|Setb_IsPlaying true)
  (if StartChoiceAfter
    (Variables|/Game/Bullied_VR/Blueprints/NEWBlueprints/BP_TextTriggerBox.BP_TextTriggerBox_C|Setb_StartChoiceAfter _texttriggerref StartChoiceAfter)
    (Variables|/Game/Bullied_VR/Blueprints/NEWBlueprints/BP_TextTriggerBox.BP_TextTriggerBox_C|SetA_Choice _texttriggerref ChoiceArray)))