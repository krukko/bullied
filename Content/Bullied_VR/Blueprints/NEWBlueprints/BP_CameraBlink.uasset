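; BP_CameraBlink simulates eye blinks in a VR game by fading the player camera.
; CloseEye starts a fade and an elapsed timer; Tick calls OpenEyes one second after the blink time has passed.
; OpenEyes fades again and resets the timer, while EndBlink only stops it.
; SceneChangeFX runs a fade of caller-supplied duration with the eye flagged open, so no automatic reopen follows.
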(event EventBeginPlay
  (Variables|Default|Setf_ElapseTime -1.0)
  (Variables|Default|Setb_EyeClosed false))

(event EventTick
  (params (DeltaSeconds :type Float%20%28single-precision%29))
  (if (>= (Variables|Default|Getf_ElapseTime) 0.0)
    (bind _output_get (Variables|Default|Setf_ElapseTime (+ (Variables|Default|Getf_ElapseTime) (Utilities|Time|GetWorldDeltaSeconds))))
    (if (>= _output_get (+ (Variables|Default|Getf_BlinkTime) 1.0))
      (if (Variables|Default|Getb_EyeClosed)
        (CallFunction|OpenEyes)))))

(fn ConstructionScript)

(fn OpenEyes
  (CameraFades|StartCameraFade :self (Game|GetPlayerCameraManager 0) :Duration (Variables|Default|Getf_BlinkTime))
  (Variables|Default|Setf_ElapseTime -1.0)
  (Variables|Default|Setb_EyeClosed false))

(fn EndBlink
  (Variables|Default|Setf_ElapseTime -1.0))

(fn CloseEye
  (CameraFades|StartCameraFade :self (Game|GetPlayerCameraManager 0) :Duration (Variables|Default|Getf_BlinkTime))
  (Variables|Default|Setf_ElapseTime 0.0)
  (Variables|Default|Setb_EyeClosed true))

(fn SceneChangeFX
  (params (OpenEyeTime :type Float%20%28single-precision%29))
  (CameraFades|StartCameraFade :self (Game|GetPlayerCameraManager 0) :Duration OpenEyeTime)
  (Variables|Default|Setf_ElapseTime 0.0)
  (Variables|Default|Setb_EyeClosed false))