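; BP_MotionController is a VR hand actor with a grab sphere for picking up nearby objects.
; GetActorNearHand selects the closest overlapping actor that implements an interface, using a stored nearest distance that it never resets.
; GrabActor would attach that actor by sending PickUpMessage with the motion controller, but its logic is not wired to run.
; The sphere's overlap event checks physics simulation on static meshes without acting on the result.
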(event OnComponentBeginOverlap(GrabSphere)
  (params (OverlappedComponent :type Primitive%20Component%20Object%20Reference) (OtherActor :type Actor%20Object%20Reference) (OtherComp :type Primitive%20Component%20Object%20Reference) (OtherBodyIndex :type Integer) (bFromSweep :type Boolean) (SweepResult :type Hit%20Result%20Structure%20%28by%20ref%29))
  (bind _asstatic_mesh_component (Utilities|Casting|CastToStaticMeshComponent OtherComp))
  (if (Physics|IsSimulatingPhysics _asstatic_mesh_component "None")
    _))

(fn ConstructionScript)

(fn GetActorNearHand
  (bind _grabsphere (Variables|Default|GetGrabSphere))
  (for _array_element (Collision|GetOverlappingActors _grabsphere "/Script/Engine.Actor" :!class /Script/Engine.PrimitiveComponent)
    (if (Utilities|DoesObjectImplementInterface _array_element 0)
      (if (< (Math|Vector|VectorLength (- (Transformation|GetActorLocation _array_element) (Transformation|GetWorldLocation _grabsphere))) (Variables|Default|GetF_nearestOverlap))
        (Variables|Default|Seta_nearestOverlappingActor _array_element)
        (Variables|Default|SetF_nearestOverlap (Math|Vector|VectorLength (- (Transformation|GetActorLocation _array_element) (Transformation|GetWorldLocation _grabsphere)))))))
  (return (Variables|Default|Geta_nearestOverlappingActor)))