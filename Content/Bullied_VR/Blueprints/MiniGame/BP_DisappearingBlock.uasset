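; Minigame platform block that repeatedly disappears and reappears at random intervals.
; Tick runs the timer while MaxAppearTime is positive, toggling visibility and collision through HidePlatform and UnHidePlatform, which each roll the next duration.
; In the last tenth of its visible time the block shrinks every frame as a warning, and its original scale returns on reappearing.
; Overlap by PlayerMCRef pauses the visible countdown until the player leaves.
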(event EventBeginPlay
  (Utilities|FlowControl|Sequence
    (:then_0
      ;[1 1 1] Set original Scale
      (Variables|Default|Setv3_OriginalScale (Class|Actor|GetActorRelativeScale3D)))
    (:then_1
      ;[1 1 1] Check if min appear time is less than 0
      (if (< (Variables|Default|GetMinAppearTime) 0.0)
        (Variables|Default|SetMinAppearTime 0.0)
        (elif (< (Variables|Default|GetMaxAppearTime) (Variables|Default|GetMinAppearTime))
          (Variables|Default|SetMaxAppearTime (+ (Variables|Default|GetMinAppearTime) 1.0)))))
    (:then_2
      ;[1 1 1] Hide Platform on start
      (bind _output_get (Variables|Default|Setb_IsHidden (Variables|Default|GetStartHidden?)))
      (if _output_get
        (CallFunction|HidePlatform)
        (else
          (Variables|Default|Setf_AppearTime (Math|Random|RandomFloatinRange (Variables|Default|GetMinAppearTime) (Variables|Default|GetMaxAppearTime))))))))

(event EventTick
  (params (DeltaSeconds :type Float%20%28single-precision%29))
  (if (> (Variables|Default|GetMaxAppearTime) 0.0)
    (if (Variables|Default|Getb_IsHidden)
      ;[1 1 1] Update Hidden
      (bind _output_get (Variables|Default|Setf_ElapseTime (+ (Variables|Default|Getf_ElapseTime) (Utilities|Time|GetWorldDeltaSeconds))))
      (if (>= _output_get (Variables|Default|Getf_HideTime))
        (CallFunction|UnHidePlatform))
      (elif (not (Variables|Default|Getb_SteppedOn))
        ;[1 1 1] Update UnHidden
        (bind _output_get_2 (Variables|Default|Setf_ElapseTime (+ (Variables|Default|Getf_ElapseTime) (Utilities|Time|GetWorldDeltaSeconds))))
        (if (>= _output_get_2 (* (Variables|Default|Getf_AppearTime) 0.9))
          (Transformation|SetActorRelativeScale3D (* (Class|Actor|GetActorRelativeScale3D) 0.9))
          (if (>= (Variables|Default|Getf_ElapseTime) (Variables|Default|Getf_AppearTime))
            (CallFunction|HidePlatform)))))))

(event Collision|EventActorBeginOverlap
  (params (OtherActor :type Actor%20Object%20Reference))
  (bind _playermc_ref (Variables|Default|GetPlayerMC_Ref))
  (Utilities|IsValid _playermc_ref
    (:Is%20Valid
      (if (== OtherActor _playermc_ref)
        (Variables|Default|Setb_SteppedOn true)))))

(event Collision|EventActorEndOverlap
  (params (OtherActor :type Actor%20Object%20Reference))
  (bind _playermc_ref (Variables|Default|GetPlayerMC_Ref))
  (Utilities|IsValid _playermc_ref
    (:Is%20Valid
      (if (== OtherActor _playermc_ref)
        (Variables|Default|Setb_SteppedOn false)))))

(fn ConstructionScript)

(fn HidePlatform
  (Variables|Default|Setf_HideTime (Math|Random|RandomFloatinRange 0.0 (Variables|Default|GetMaxHiddenTime)))
  (Rendering|SetActorHiddenInGame true)
  (Collision|SetActorEnableCollision false)
  (Variables|Default|Setb_IsHidden true)
  (Variables|Default|Setf_ElapseTime 0.0))

(fn UnHidePlatform
  (Variables|Default|Setf_AppearTime (Math|Random|RandomFloatinRange (Variables|Default|GetMinAppearTime) (Variables|Default|GetMaxAppearTime)))
  (Transformation|SetActorRelativeScale3D (Variables|Default|Getv3_OriginalScale))
  (Rendering|SetActorHiddenInGame false)
  (Collision|SetActorEnableCollision true)
  (Variables|Default|Setb_IsHidden false)
  (Variables|Default|Setf_ElapseTime 0.0))