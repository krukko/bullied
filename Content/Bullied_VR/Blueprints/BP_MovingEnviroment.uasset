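; BP_MovingEnviroment is an actor that scrolls along a straight path in a repeating loop while IsMoving is true.
; BeginPlay stores the starting location and derives the end point by flipping and shrinking its world Y coordinate.
; Tick moves it a fixed step per frame toward that point, without delta-time scaling.
; It snaps back to the start once the next step's Y reaches or exceeds the end point's.
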(event EventBeginPlay
  (bind _output_get (Variables|Default|SetOriginalPoint (Transformation|GetActorLocation)))
  (Variables|Default|SetEndPoint (* _output_get "1.000000,-0.330000,1.000000")))

(event EventTick
  (params (DeltaSeconds :type Float%20%28single-precision%29))
  (bind _returnvalue (Transformation|GetActorLocation))
  (bind _originalpoint (Variables|Default|GetOriginalPoint))
  (bind _endpoint (Variables|Default|GetEndPoint))
  (bind _returnvalue_2 (- _endpoint _originalpoint))
  (bind _returnvalue_3 (Math|Vector|Normalize _returnvalue_2))
  (bind _returnvalue_4 (* _returnvalue_3 15.0))
  (bind _returnvalue_5 (+ _returnvalue _returnvalue_4))
  (if (Variables|Default|GetIsMoving)
    (Transformation|SetActorLocation _returnvalue_5 false false)
    (if (>= (.Y (Math|Vector|BreakVector _returnvalue_5)) (.Y (Math|Vector|BreakVector (Variables|Default|GetEndPoint))))
      (Transformation|SetActorLocation (Variables|Default|GetOriginalPoint) false false))))

(fn ConstructionScript)