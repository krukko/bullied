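; BP_CamEffectCollisionBox is a trigger volume in the Bullied VR project that closes the player's eyes through a blink effect.
; Each Tick it polls whether CollisionBox overlaps PlayerMCRef and, if so, calls CloseEye on BlinkRef once, latched by BTriggered.
; Any actor ending overlap clears the latch without a filter, and nothing here reopens the eye.
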(event EventBeginPlay)

(event Collision|EventActorBeginOverlap
  (params (OtherActor :type Actor%20Object%20Reference)))

(event Collision|EventActorEndOverlap
  (params (OtherActor :type Actor%20Object%20Reference))
  (Variables|Default|Setb_Triggered false))

(event EventTick
  (params (DeltaSeconds :type Float%20%28single-precision%29))
  (if (and (Collision|IsOverlappingActor (Variables|Default|GetCollisionBox) (Variables|Default|GetPlayerMCRef) :!class /Script/Engine.PrimitiveComponent) (not (Variables|Default|Getb_Triggered)))
    (Default|CloseEye (Variables|Default|GetBlinkRef))
    (Variables|Default|Setb_Triggered true)))

(fn ConstructionScript)