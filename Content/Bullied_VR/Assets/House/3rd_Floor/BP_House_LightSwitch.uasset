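; VR light switch Blueprint for the house that toggles its assigned ceiling and stair lights when a player's motion controller touches it.
; Tick polls the box collision against the left, then right controller while the HandsOff latch is set.
; A touch clears the latch, toggles both light arrays, rumbles that controller and plays a sound at the switch.
; Any actor end-overlap event re-arms the latch.
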(event EventBeginPlay
  (Variables|Default|SetHandsOff true))

(event Collision|EventActorBeginOverlap
  (params (OtherActor :type Actor%20Object%20Reference)))

(event EventTick
  (params (DeltaSeconds :type Float%20%28single-precision%29))
  (bind _ceiling_lights (Variables|Default|GetCeiling%20Lights))
  (bind _playermotioncontrollerref (Variables|Default|GetPlayerMotionControllerRef))
  (bind _stair_lights (Variables|Default|GetStair%20Lights))
  (bind _rightcontroller (Variables|/Game/Bullied_VR/Blueprints/Player/BP_MotionControllerPawnFPS.BP_MotionControllerPawnFPS_C|GetRightController _playermotioncontrollerref))
  (bind _leftcontroller (Variables|/Game/Bullied_VR/Blueprints/Player/BP_MotionControllerPawnFPS.BP_MotionControllerPawnFPS_C|GetLeftController _playermotioncontrollerref))
  ;[1 1 1] Switch Collision with Player
  (if (Variables|Default|GetHandsOff)
    (if (Collision|IsOverlappingActor (Variables|Default|GetBoxCollision) _leftcontroller :!class /Script/Engine.PrimitiveComponent)
      (Variables|Default|SetHandRef _leftcontroller)
      (Variables|Default|SetHandsOff false :!label _label)
      (Utilities|FlowControl|Sequence
        (:then_0
          (if (> (Utilities|Array|Length _ceiling_lights) 0)
            (for _array_element _ceiling_lights
              (Default|LightsToggle _array_element))))
        (:then_1
          (if (> (Utilities|Array|Length _stair_lights) 0)
            (for _array_element_2 _stair_lights
              (Default|LightsToggle _array_element_2))))
        (:then_2
          (Default|RumbleController (Variables|Default|GetHandRef) 0.5)
          (Audio|PlaySoundatLocation 0 (Transformation|GetWorldLocation (Variables|Default|GetSwitch)) "0, 0, 0" 1.0 1.0 0.0 0 0 0)))
      (elif (Collision|IsOverlappingActor (Variables|Default|GetBoxCollision) _rightcontroller :!class /Script/Engine.PrimitiveComponent)
        (Variables|Default|SetHandRef _rightcontroller)
        (goto _label)))))

(event Collision|EventActorEndOverlap
  (params (OtherActor :type Actor%20Object%20Reference))
  (Variables|Default|SetHandsOff true))

(fn ConstructionScript)