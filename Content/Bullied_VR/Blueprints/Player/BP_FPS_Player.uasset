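; First-person player pawn for Bullied_VR, with axis-driven look and movement plus gaze-based interaction.
; Each tick, a camera line trace moves a VisionTrigger volume to the hit point, or back to the mesh on a miss.
; Overlapping lookable actors build a dwell timer that calls LookTriggerMessage through their interface after about two seconds.
; BeginPlay touches subtitle and choice HUD variables; trigger master-player assignments and FPS text are disconnected.
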(event EventTick
  (params (DeltaSeconds :type Float%20%28single-precision%29))
  (bind _camera (Variables|Default|GetCamera))
  (bind _visiontrigger (Variables|Default|GetVisionTrigger))
  (bind _returnvalue (Transformation|GetWorldLocation _camera))
  (Utilities|FlowControl|Sequence
    (:then_0
      ;[1 1 1] Sight trigger for interactable actors
      (bind (_outhit _returnvalue_2) (Collision|LineTraceByChannel _returnvalue (+ _returnvalue (* (Math|Vector|GetForwardVector _camera) (Variables|Default|Getf_LookableDistance))) "TraceTypeQuery1" false 0 "None" true "(R=1.000000,G=0.000000,B=0.000000,A=1.000000)" "(R=0.000000,G=1.000000,B=0.000000,A=1.000000)" DeltaSeconds))
      (if _returnvalue_2
        (Transformation|SetWorldLocation _visiontrigger (.ImpactPoint (Collision|BreakHitResult _outhit)) false false)
        (bind _array_element (Utilities|Array|ForEachLoopwithBreak (Collision|GetOverlappingActors _visiontrigger "/Game/Bullied_VR/Blueprints/BP_LookableActor.BP_LookableActor_C" :!class /Script/Engine.PrimitiveComponent) :!label _label)
          (:LoopBody
            (bind _asbp_interface_lookable (Utilities|Casting|CastToBP_InterfaceLookable _array_element)
              (:then
                (bind _output_get (Variables|Default|SetLos_Interactable_Actor _asbp_interface_lookable))
                (bind _output_get_2 (Variables|Default|Setf_elapsed_Time (+ (Variables|Default|Getf_elapsed_Time) DeltaSeconds)))
                (Math|Float|CompareFloat _output_get_2 2.0
                  (:>
                    _)
                  (:==
                    _)
                  (:<
                    (goto _label Break)))
                (Class|BPInterfaceLookable|LookTrigger(Message) (Utilities|ToObject(Interface) _output_get) self))
              (:CastFailed
                _))
            (Variables|Default|Setf_elapsed_Time 0.0)
            (goto _label Break)))
        (else
          (Transformation|SetWorldLocation _visiontrigger (Transformation|GetWorldLocation (Variables|Character|GetMesh)) false false))))))

(event EventBeginPlay
  (Utilities|FlowControl|Sequence
    (:then_0
      ;[1 1 1] HUD Display
      (Variables|Default|SetSubtitles (Variables|Default|GetSubtitles))
      (Variables|Default|SetChoices (Variables|Default|GetChoices)))))

(event Input|AxisEvents|InputAxisMoveLeft
  (params (AxisValue :type Float%20%28single-precision%29))
  ;[1 1 1] Movement
  (Pawn|Input|AddMovementInput (Transformation|GetActorRightVector) AxisValue false))

(event Input|AxisEvents|InputAxisLookHorizontal
  (params (AxisValue :type Float%20%28single-precision%29))
  ;[1 1 1] Looking around
  (Pawn|Input|AddControllerYawInput AxisValue))

(event Input|AxisEvents|InputAxisLookVertical
  (params (AxisValue :type Float%20%28single-precision%29))
  ;[1 1 1] Looking around
  (Pawn|Input|AddControllerPitchInput AxisValue))

(event Input|AxisEvents|InputAxisMoveForwardBack
  (params (AxisValue :type Float%20%28single-precision%29))
  ;[1 1 1] Movement
  (Pawn|Input|AddMovementInput (Transformation|GetActorForwardVector) AxisValue false))

(fn ConstructionScript)