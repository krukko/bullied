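; AI controller for the female NPC that feeds a looping waypoint patrol to its behavior tree.
; On BeginPlay it runs BT_FemaleNPC, caches the controlled Female_NPC and its waypoint count, requests the first waypoint, then records the pawn's start location.
; Each NextWaypoint call writes the next WaypointArray entry to the TargetLocation blackboard key, or the start location once the array is exhausted, resetting the index to restart the loop.
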(event Custom|NextWaypoint
  (bind _returnvalue (Utilities|Name|MakeLiteralName "TargetLocation"))
  (bind _returnvalue_2 (AI|GetBlackboard 0))
  (Math|Integer|CompareInt (Variables|Default|GetWaypointIndex) (Variables|Default|GetWaypointLength)
    (:==
      (AI|Components|Blackboard|SetValueasVector _returnvalue_2 _returnvalue (Variables|Default|GetStartLocation))
      (Variables|Default|SetWaypointIndex 0))
    (:<
      (AI|Components|Blackboard|SetValueasVector _returnvalue_2 _returnvalue (Utilities|Array|Get(acopy) (Variables|/Game/Bullied_VR/Blueprints/NPC_BPs/Female_NPC.Female_NPC_C|GetWaypointArray (Variables|Default|GetControlledNPC)) (Variables|Default|GetWaypointIndex)))
      (Math|Integer|IncrementInt (Variables|Default|GetWaypointIndex)))))

(event EventBeginPlay
  (bind _returnvalue (Pawn|GetControlledPawn))
  (AI|RunBehaviorTree "/Game/Bullied_VR/Blueprints/NPC_BPs/BT_FemaleNPC.BT_FemaleNPC")
  (bind _asfemale_npc (Utilities|Casting|CastToFemale_NPC _returnvalue))
  (Variables|Default|SetControlledNPC _asfemale_npc)
  (Variables|Default|SetWaypointLength (Utilities|Array|Length (Variables|/Game/Bullied_VR/Blueprints/NPC_BPs/Female_NPC.Female_NPC_C|GetWaypointArray _asfemale_npc)))
  (CallFunction|NextWaypoint)
  (Variables|Default|SetStartLocation (Transformation|GetActorLocation _returnvalue)))

(fn ConstructionScript)