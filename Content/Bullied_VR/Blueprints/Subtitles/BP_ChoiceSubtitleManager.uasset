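; Manager actor that runs subtitle sequences and dialogue choices for the VR pawn, BP_MotionControllerPawnFPS.
; ActivateSubtitle starts the TTB text box and can queue a follow-up choice, while ActivateChoice opens the CTB choice box directly.
; A Delay-throttled Tick polls the pawn's left-hand input outside cutscenes, routing trigger and scroll to choice selection or trigger to text advance, then clears CSMDoAction to consume the input.
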(event EventBeginPlay
  (bind _outactors (Actor|GetAllActorsOfClass "/Game/Bullied_VR/Blueprints/Player/BP_MotionControllerPawnFPS.BP_MotionControllerPawnFPS_C"))
  (bind _array_element (Utilities|Array|ForEachLoopwithBreak _outactors :!label _label)
    (:LoopBody
      (Variables|Default|SetPlayer%20Ref _array_element)
      (goto _label Break))))

(event Collision|EventActorBeginOverlap
  (params (OtherActor :type Actor%20Object%20Reference)))

(event EventTick
  (params (DeltaSeconds :type Float%20%28single-precision%29))
  (bind _player_ref (Variables|Default|GetPlayer%20Ref))
  (bind _ctb (Variables|Default|GetCTB))
  (bind _ttb (Variables|Default|GetTTB))
  (bind _triggerleft_down (Variables|/Game/Bullied_VR/Blueprints/Player/BP_MotionControllerPawnFPS.BP_MotionControllerPawnFPS_C|GetTriggerLeft_Down _player_ref))
  (Utilities|FlowControl|Delay 0.1)
  (if (Variables|/Game/Bullied_VR/Blueprints/Player/BP_MotionControllerPawnFPS.BP_MotionControllerPawnFPS_C|GetCSM_DoAction _player_ref)
    (if (not (Variables|/Game/Bullied_VR/Blueprints/Triggers/CurrentlyInGame_OriginalBPs/BP_Text_Trigger_Box.BP_Text_Trigger_Box_C|GetIsPlayingCutscene _ttb))
      (if (Variables|/Game/Bullied_VR/Blueprints/Player/BP_MotionControllerPawnFPS.BP_MotionControllerPawnFPS_C|GetInChoice _player_ref)
        (Utilities|FlowControl|Sequence
          (:then_0
            (if _triggerleft_down
              (Default|SelectChoice _ctb)
              (Variables|/Game/Bullied_VR/Blueprints/Player/BP_MotionControllerPawnFPS.BP_MotionControllerPawnFPS_C|SetCSM_DoAction _player_ref false :!label _label)))
          (:then_1
            (if (Variables|/Game/Bullied_VR/Blueprints/Player/BP_MotionControllerPawnFPS.BP_MotionControllerPawnFPS_C|GetScrollUp_Left _player_ref)
              (Default|ChangeChoiceUp _ctb)
              (goto _label)))
          (:then_2
            (if (Variables|/Game/Bullied_VR/Blueprints/Player/BP_MotionControllerPawnFPS.BP_MotionControllerPawnFPS_C|GetScrollDown_Left _player_ref)
              (Default|ChangeChoiceDown _ctb)
              (goto _label))))
        (elif (Variables|/Game/Bullied_VR/Blueprints/Triggers/CurrentlyInGame_OriginalBPs/BP_Text_Trigger_Box.BP_Text_Trigger_Box_C|GetIsInteracting _ttb)
          (if _triggerleft_down
            (Default|IterateText _ttb)
            (goto _label)))))))

(fn ConstructionScript)

(fn ActivateChoice
  (params (Choice :type Array%20of%20Choice%20Info%20Structures) (Disable%20Motion :type Boolean))
  (Default|StartChoiceSelection (Variables|Default|GetCTB) Choice Disable%20Motion)
  (Variables|Default|SetIsPlaying true))

(fn ActivateSubtitle
  (params (Subtitle :type Subtitle%20Info%20Structure) (StartChoiceAfter :type Boolean) (ChoiceArray :type Array%20of%20Choice%20Info%20Structures) (DisableMotion :type Boolean) (CurrEventTBox :type BP%20Event%20Trigger%20Box%20Object%20Reference))
  (bind _ttb (Variables|Default|GetTTB))
  (Default|StartSubtitleSequence _ttb Subtitle DisableMotion)
  (Variables|Default|SetCurrEventTBox CurrEventTBox)
  (Variables|Default|SetIsPlaying true)
  (if StartChoiceAfter
    (Variables|/Game/Bullied_VR/Blueprints/Triggers/CurrentlyInGame_OriginalBPs/BP_Text_Trigger_Box.BP_Text_Trigger_Box_C|SetStartChoiceAfter _ttb StartChoiceAfter)
    (Variables|/Game/Bullied_VR/Blueprints/Triggers/CurrentlyInGame_OriginalBPs/BP_Text_Trigger_Box.BP_Text_Trigger_Box_C|SetChoiceArray _ttb ChoiceArray)))